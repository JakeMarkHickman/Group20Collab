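; Tutorial trigger that shows the player a pop-up explaining the rat's four abilities and their keyboard and d-pad controls.
; When the first player's controlled pawn begins overlapping the collision component, it creates a tutorial pop-up widget, adds it to the viewport and fills both text fields with hardcoded copy.
; Any end overlap on that component destroys the trigger actor, without checking which actor left.
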(event `self.CollisionComponent.OnComponentBeginOverlap`
  (params (OverlappedComponent :type "PrimitiveComponent Object Reference") (OtherActor :type "Actor Object Reference") (OtherComp :type "PrimitiveComponent Object Reference") (OtherBodyIndex :type Integer) (bFromSweep :type Boolean) (SweepResult :type "HitResult Structure (by ref)"))
  ;[1 1 1] show pop up
  (if (== OtherActor (`Controller.K2_GetPawn` (`GameplayStatics.GetPlayerController` 0)))
    (bind _returnvalue (`|CreateWidget` "/Game/Tutorialisation/T_UI/WBP_tutorialPopUp.WBP_tutorialPopUp_C" (`self.player con`)))
    (`UserWidget.AddToViewport` _returnvalue 0)
    (`TextBlock.SetText` (`/Game/Tutorialisation/T_UI/WBP_tutorialPopUp.txt_1` _returnvalue) "As the rat, you have four abilities: \nFlea Bomb - will release fleas to confuse villagers.  \nRat Allies - will release a stun that will stall villagers for a few seconds. \nStun - Spawn rats at your side, which will infect another villager for you. \nSqueak - will make a noise to draw villagers towards you")
    (`TextBlock.SetText` (`/Game/Tutorialisation/T_UI/WBP_tutorialPopUp.txt_2` _returnvalue) "The controls for these are: \n1/d-pad up - Flea Bomb \n2/d-pad right. Rat Allies \n3/d-pad down - Stun \n4/d-pad left - Squeak")))

(event `self.CollisionComponent.OnComponentEndOverlap`
  (params (OverlappedComponent :type "PrimitiveComponent Object Reference") (OtherActor :type "Actor Object Reference") (OtherComp :type "PrimitiveComponent Object Reference") (OtherBodyIndex :type Integer))
  ;[1 1 1] destroy collision
  (`self.K2_DestroyActor`))

(fn `UserConstructionScript`)