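; SE_Slowness is a status effect that slows the afflicted actor's walking speed.
; On start it caches the actor's CharacterMovementComponent and current MaxWalkSpeed, then scales that speed down to 40%.
; On end it writes the cached speed back, overwriting any change made to MaxWalkSpeed while the effect was active.
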(event `self.StartStatusEffect`
  (params (Afflicted :type "Actor Object Reference"))
  (bind _character_movement (`self.Character movement`))
  (bind _maxwalkspeed (`CharacterMovementComponent.MaxWalkSpeed` _character_movement))
  (set `self.Character movement` (`Actor.GetComponentByClass` Afflicted "/Script/Engine.CharacterMovementComponent"))
  (set `self.Max Walk Speed` _maxwalkspeed)
  (set `CharacterMovementComponent.MaxWalkSpeed` (* _maxwalkspeed 0.4) _character_movement))

(event `self.EndStatusEffect`
  (set `CharacterMovementComponent.MaxWalkSpeed` (`self.Max Walk Speed`) (`self.Character movement`)))