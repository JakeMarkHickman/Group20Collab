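; BP_MainMenuRat is a rat character, named for the main menu, with biting, sprinting and death handling.
; Bite sphere-traces forward from the mesh, then damages and infects villagers it hits, while sprint calls forward to a component.
; Death reloads Level0 when in that level, otherwise signals game lost through the gamemode.
; A debug key toggles a villager between attacking and passive; BeginPlay, UseAbility and the disconnected ability-level setup do nothing.
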(event OnDeath(Health)
  (params (Instigator :type Controller%20Object%20Reference))
  ;[1 1 1] respawn in tutorial level
  (bind _returnvalue (Game|GetCurrentLevelName true))
  (if (Utilities|Enum|Equal(Enum) _returnvalue "Level0")
    (Game|OpenLevel(byObjectReference) "/Game/Levels/Level0.Level0")
    (else
      (bind _asbp_rat_gamemode (Utilities|Casting|CastToBP_RatGamemode (Game|GetGameMode)))
      (Default|CallEGameLost _asbp_rat_gamemode))))

(event EventStartSprint
  ;[1 1 1] Sprinting
  (Default|StartSprint (Variables|Default|GetBPC_Sprint)))

(event EventEndSprint
  ;[1 1 1] Sprinting
  (Default|EndSprint (Variables|Default|GetBPC_Sprint)))

(event EventUseAbility)

(event EventBiteAction
  (CallFunction|Bite 5e+01 2e+01))

(event EventBeginPlay)

(event Input|KeyboardEvents|DebugKey1
  (params (Key :type Key%20Structure :default "None") (ActionValue :type Input%20Action%20Value%20Structure))
  (:Pressed
    (bind _returnvalue (Actor|GetActorOfClass "/Game/Blueprints/AI/Pawns/BP_Villager.BP_Villager_C"))
    (bind _asaic_villager (Utilities|Casting|CastToAIC_Villager (AI|GetAIController _returnvalue)))
    (Utilities|FlowControl|FlipFlop
      (:A
        (Default|SetStateasAttacking _asaic_villager self false))
      (:B
        (Default|SetStateasPassive _asaic_villager)))))

(fn ConstructionScript)

(fn Bite
  (params (BiteRange :type Float%20%28double-precision%29) (BiteRadius :type Float%20%28double-precision%29))
  (bind _mesh (Variables|Character|GetMesh))
  (bind _returnvalue (Transformation|GetWorldLocation _mesh))
  (bind _outhits (Collision|MultiSphereTraceForObjects _returnvalue (+ _returnvalue (* (Math|Rotator|GetRotationXVector (Transformation|GetWorldRotation _mesh)) (Math|Vector|MakeVector BiteRange BiteRange 0.0))) BiteRadius (Utilities|Array|MakeArray "ObjectTypeQuery3") false 0 "None"))
  (for _array_element _outhits
    ;[1 1 1] Check if Actor is a Villager
    (if (== (Utilities|GetClass (.HitActor (Collision|BreakHitResult _array_element))) "/Game/Blueprints/AI/Pawns/BP_Villager.BP_Villager_C")
      ;[1 1 1] Set AI as Damaged
      (Class|BPIAI|SetStateasDamaged(Message) (.HitActor (Collision|BreakHitResult _array_element)))
      ;[1 1 1] Add Status effect here
      (Class|StatusEffectComponent|AddStatusEffect (Actor|GetComponentbyClass (Pawn|GetControlledPawn (AI|GetAIController (.HitActor (Collision|BreakHitResult _array_element)))) "/Script/Group20Collab.StatusEffectComponent") "/Game/Blueprints/StatusEffects/SE_Infected1.SE_Infected1_C")
      (Audio|PlaySoundatLocation "/Game/Assets/Audio/Rat_Audio/RatBite_-_Track_10.RatBite_-_Track_10" (Transformation|GetActorLocation) "0, 0, 0" 4.0 1.0 0.0 0 0 0 0))))