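; Base projectile actor that travels to a target location and infects nearby pawns on arrival, apparently with fleas.
; Initialise stores the target, then a timeline lerps the actor from its current position toward it each update, without sweeping.
; On finish, a debug-drawn sphere trace of flea range gives each hit pawn with a valid GetRefVMessage reference the SE_Infected1 status effect.
; An unconnected random switch into the infection step never runs.
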(event `Initialise`
  (params (Location :type "Vector Structure"))
  (set `self.Location` Location)
  (`self.Move`))

(event `Move`
  (bind _location (`self.Location`))
  (bind (_direction _moveto) (`Timeline|Timeline`)
    (:`Update`
      (`self.K2_SetActorLocation` (`KismetMathLibrary.VLerp` (`self.K2_GetActorLocation`) (`self.Location`) _moveto)))
    (:`Finished`
      (bind _outhits (`KismetSystemLibrary.SphereTraceMultiForObjects` :`Start` _location :`End` _location :`Radius` (`self.FleaRange`) :`ObjectTypes` (`|MakeArray` "ObjectTypeQuery3" :!type "EObjectTypeQuery Enum") :`DrawDebugType` "Persistent"))
      (for _array_element _outhits
        (bind (_bblockinghit _binitialoverlap _time _distance _location_2 _impactpoint _normal _impactnormal _physmat _hitactor) (`GameplayStatics.BreakHitResult` _array_element))
        (`KismetSystemLibrary.PrintString` (`KismetSystemLibrary.GetDisplayName` _hitactor))
        (bind _bp_villager (message `/Game/Blueprints/AI/Interfaces/BPI_AI.GetRef_V` _hitactor))
        (`/Engine/EditorBlueprintResources/StandardMacros.IsValid` _bp_villager
          (:`Is Valid`
            (`StatusEffectComponent.AddStatusEffect` (`/Game/Blueprints/AI/Pawns/BP_Villager.StatusEffect` _bp_villager) "/Game/Blueprints/StatusEffects/SE_Infected1.SE_Infected1_C")
            (`KismetSystemLibrary.PrintString` "Infected"))
          (:`Is Not Valid`
            (`KismetSystemLibrary.PrintString` "Not Infectable")))))))

(fn `UserConstructionScript`)