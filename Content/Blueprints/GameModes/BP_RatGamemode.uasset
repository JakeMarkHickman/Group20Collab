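; Game mode for a rat plague level: the player wins when all villagers are infected or dead and loses when the rat dies.
; Villager death events trigger a recount that either records completion with fixed three stars or spawns an AI plague doctor.
; The recount also drives a timeline that tilts the directional light between start and end pitch by the fraction of villagers still alive.
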(event `self.ReceiveBeginPlay`
  ;[1 1 1] Init
  (bind _outactors (`GameplayStatics.GetAllActorsOfClass` "/Game/Blueprints/AI/Pawns/BP_Villager.BP_Villager_C"))
  (set `self.TotalVillagersInLevel` _outactors)
  (bind _returnvalue (`GameplayStatics.GetActorOfClass` "/Script/Engine.DirectionalLight"))
  (set `self.DirectionalLight` _returnvalue)
  (add `self.E_VillagerDied` (`|CreateDelegate` :!event `UpdateVillagerNumbers`))
  (add `self.E_RatDied` (`|CreateDelegate` :!event `UpdateOnRatDeath`))
  (`self.SetSunRotation` (`self.StartSunRotation`))
  (`self.UpdateVillagerNumbers`))

(event `UpdateVillagerNumbers`
  (bind _spawn_transform (`self.Spawn Transform`))
  ;[1 1 1] Updating and Checking Villager Numbers
  (`KismetArrayLibrary.Array_Clear` (`self.InfectedVillagersInLevel`))
  (`KismetArrayLibrary.Array_Clear` (`self.AliveVillagersInLevel`))
  (bind _outactors (`GameplayStatics.GetAllActorsOfClass` "/Game/Blueprints/AI/Pawns/BP_Villager.BP_Villager_C"))
  (for _array_element _outactors
    (`|ExecutionSequence`
      (:`then_0`
        ;;[1 0 0] ADD INFECTED STATUS EFFECT
        (if (`KismetArrayLibrary.Array_Contains` (`StatusEffectComponent.GetActiveStatusEffects` (`/Game/Blueprints/AI/Pawns/BP_Villager.StatusEffect` _array_element)))
          (`KismetArrayLibrary.Array_Add` (`self.InfectedVillagersInLevel`) _array_element :!label _label)))
      (:`then_1`
        (if (`HealthComponent.GetIsDead` (`self.GetComponentByClass` _array_element "/Script/Group20Collab.HealthComponent"))
          (goto _label)
          (else
            (`KismetArrayLibrary.Array_Add` (`self.AliveVillagersInLevel`) _array_element)
            (`self.SunRotationUpdate`))))))
  ;[1 1 1] Sun Rotation Update
  (`KismetSystemLibrary.PrintString` (`KismetStringLibrary.Concat_StrStr` (`KismetStringLibrary.Conv_IntToString` (`KismetArrayLibrary.Array_Length` (`self.InfectedVillagersInLevel`))) " villagers left to infect"))
  (if (`KismetArrayLibrary.Array_Identical` (`self.InfectedVillagersInLevel`) (`self.TotalVillagersInLevel`))
    (`KismetSystemLibrary.PrintString` "Hello")
    (`self.E_GameWon` (`KismetSystemLibrary.GetGameTimeInSeconds`))
    ;[1 1 1] UpdateLevelInstance (Needs stars)
    (bind _returnvalue (`GameplayStatics.GetCurrentLevelName` true))
    (message `/Game/UI/BPI_UI.UpdateLevelInstance` (`GameplayStatics.GetGameInstance`) _returnvalue true 3)
    (else
      (bind _returnvalue_2 (`|SpawnActorFromClass` "/Game/Blueprints/AI/Controllers/AIC_PlagueDoctor.AIC_PlagueDoctor_C" _spawn_transform "Undefined" "MultiplyWithRoot" null null))
      (`|SpawnActorFromClass` "/Game/Blueprints/AI/Pawns/BP_PlagueDoctor.BP_PlagueDoctor_C" _spawn_transform "Undefined" "MultiplyWithRoot" _returnvalue_2 "/Game/Blueprints/Weapons/BP_Weapon.BP_Weapon_C" null 50.0 null))))

(event `UpdateOnRatDeath`
  ;[1 1 1] When rat dies, lose
  (`self.E_GameLost`))

(event `SunRotationUpdate`
  (bind (_returnvalue_roll _returnvalue_pitch) (`KismetMathLibrary.BreakRotator` (`SceneComponent.K2_GetComponentRotation` (`Light.LightComponent` (`self.DirectionalLight`)))))
  ;[1 1 1] Sun Rotation Update
  (set `self.CurrentWorldRotation` _returnvalue_pitch)
  (bind _newrotationvalue (`self.CalculateLightRotation`))
  (bind (_direction _alpha) (`Timeline|SunRotation` :!via `PlayFromStart`)
    (:`Update`
      (`self.SetSunRotation` (`KismetMathLibrary.Lerp` (`self.CurrentWorldRotation`) _newrotationvalue _alpha)))))

(fn `CalculateLightRotation`
  (returns (NewRotationValue :type "Float (double-precision)"))
  (return (`KismetMathLibrary.Lerp` (`self.EndSunRotation`) (`self.StartSunRotation`) (/ (`KismetArrayLibrary.Array_Length` (`self.AliveVillagersInLevel`)) (`KismetArrayLibrary.Array_Length` (`self.TotalVillagersInLevel`))))))

(fn `SetSunRotation`
  (params (RotationPitchValue :type "Float (double-precision)"))
  (`SceneComponent.K2_SetWorldRotation` (`Light.LightComponent` (`self.DirectionalLight`)) (`KismetMathLibrary.MakeRotator` 0.0 RotationPitchValue) false false))

(fn `UserConstructionScript`)