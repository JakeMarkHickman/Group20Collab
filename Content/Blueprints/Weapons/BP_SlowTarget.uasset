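; Smoke bomb area actor that applies a slowness status effect to targets around it.
; On BeginPlay it spawns an enlarged smoke Niagara effect above itself and sphere-traces nearby pawns, adding SE_Slowness to those with a StatusEffectComponent.
; Afterward, its Sphere overlap adds the same effect only when the entering actor matches BPRat, without checking that the component exists.
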(event `self.ReceiveBeginPlay`
  (bind _returnvalue (`self.K2_GetActorLocation`))
  (`NiagaraFunctionLibrary.SpawnSystemAtLocation` "/Game/Particles/N_SmokeBomb.N_SmokeBomb" (+ (`self.K2_GetActorLocation`) (0.0 0.0 200.0)) (struct) (2.0 2.0 2.0))
  (bind _outhits (`KismetSystemLibrary.SphereTraceMultiForObjects` _returnvalue _returnvalue 400.0 (`|MakeArray` "ObjectTypeQuery3" :!type "EObjectTypeQuery Enum")))
  (for _array_element _outhits
    (bind _returnvalue_2 (`self.GetComponentByClass` (`.HitActor` (`GameplayStatics.BreakHitResult` _array_element)) "/Script/Group20Collab.StatusEffectComponent"))
    (if (!= _returnvalue_2 null)
      (`StatusEffectComponent.AddStatusEffect` _returnvalue_2 "/Game/Blueprints/StatusEffects/SE_Slowness.SE_Slowness_C"))))

(event `Initialise`)

(event `self.Sphere.OnComponentBeginOverlap`
  (params (OverlappedComponent :type "PrimitiveComponent Object Reference") (OtherActor :type "Actor Object Reference") (OtherComp :type "PrimitiveComponent Object Reference") (OtherBodyIndex :type Integer) (bFromSweep :type Boolean) (SweepResult :type "HitResult Structure (by ref)"))
  (if (== (`self.BP_Rat`) OtherActor)
    (`StatusEffectComponent.AddStatusEffect` (`self.GetComponentByClass` OtherActor "/Script/Group20Collab.StatusEffectComponent") "/Game/Blueprints/StatusEffects/SE_Slowness.SE_Slowness_C")))

(fn `UserConstructionScript`)