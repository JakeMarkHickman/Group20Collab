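; Rat repellant grenade projectile that is lobbed at an attack target and leaves a slow effect where it hits.
; On BeginPlay it ignores its owner for collision and computes a moving-target launch velocity from the owner's location, offsetting the aim by the target's velocity.
; On hit it spawns BP_SlowTarget below the hit location, passing along its rat reference, then destroys itself next tick.
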(event `self.ReceiveBeginPlay`
  (bind _attacktarget (`self.AttackTarget`))
  (`PrimitiveComponent.IgnoreActorWhenMoving` (`self.SphereCollision`) (`self.GetOwner`) true)
  (bind _outlaunchvelocity (`GameplayStatics.SuggestProjectileVelocity_MovingTarget` (`self.K2_GetActorLocation` (`self.GetOwner`)) _attacktarget (`self.GetVelocity` _attacktarget) 0.0 1.0 "None"))
  (set `MovementComponent.Velocity` _outlaunchvelocity (`self.ProjectileMovement`)))

(event `self.ReceiveHit`
  (params (MyComp :type "PrimitiveComponent Object Reference") (Other :type "Actor Object Reference") (OtherComp :type "PrimitiveComponent Object Reference") (bSelfMoved :type Boolean) (HitLocation :type "Vector Structure") (HitNormal :type "Vector Structure") (NormalImpulse :type "Vector Structure") (Hit :type "HitResult Structure (by ref)"))
  (`|SpawnActorFromClass` "/Game/Blueprints/Weapons/BP_SlowTarget.BP_SlowTarget_C" (`KismetMathLibrary.MakeTransform` (- HitLocation (0.0 0.0 150.0))) "AlwaysSpawn" "MultiplyWithRoot" null (`self.BP_Rat`) null)
  (`KismetSystemLibrary.DelayUntilNextTick`)
  (`self.K2_DestroyActor`))

(fn `UserConstructionScript`)