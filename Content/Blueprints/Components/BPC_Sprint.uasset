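; Sprint component that raises the owner's CharacterMovement max walk speed while sprinting and manages a stamina pool.
; StartSprint requires movement and stamina, then starts a looping timer for draining stamina.
; Ending the sprint or running out divides speed by 1.5 and starts a one-second exhaustion delay before gradual regeneration.
; Stamina changes broadcast through StaminaModified, with all updates driven by timers rather than Tick.
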(event `self.ReceiveBeginPlay`
  ;[1 1 1] Initialisation
  (set `self.MovementComponent` (`Actor.GetComponentByClass` (`self.GetOwner`) "/Script/Engine.CharacterMovementComponent")))

(event `/Game/Blueprints/Interfaces/BPI_Sprint.StartSprint`
  ;[1 1 1] Start Sprinting
  (set `self.Button?` true)
  (if (> (`KismetMathLibrary.VSize` (`MovementComponent.Velocity` (`self.MovementComponent`))) 0.0)
    (if (== (`self.CurrentStamina`) 0.0)
      (set `self.Sprinting?` false :!label _label)
      (else
        (set `CharacterMovementComponent.MaxWalkSpeed` 900.0 (`self.MovementComponent`))
        (bind _returnvalue (`KismetSystemLibrary.K2_SetTimerDelegate` (`|CreateDelegate` :!event `DecreaseStamina`) 0.1 true))
        (set `self.DecreaseStaminaTimerHandle` _returnvalue)
        (`KismetSystemLibrary.K2_ClearAndInvalidateTimerHandle` (`self.RegainStaminaTimerHandle`))
        (set `self.Sprinting?` true)
        (`self.StaminaModified` (`self.CurrentStamina`) (`self.MaxStamina`))))
    (else
      (goto _label))))

(event `/Game/Blueprints/Interfaces/BPI_Sprint.EndSprint`
  (bind _movementcomponent (`self.MovementComponent`))
  ;[1 1 1] Finish Sprinting
  (set `self.Button?` false)
  (if (`self.Sprinting?`)
    (set `CharacterMovementComponent.MaxWalkSpeed` (/ (`CharacterMovementComponent.MaxWalkSpeed` _movementcomponent) 1.5) _movementcomponent)
    (`self.FinishStamina`)
    (`KismetSystemLibrary.K2_ClearAndInvalidateTimerHandle` (`self.DecreaseStaminaTimerHandle`))))

(event `self.ReceiveTick`
  (params (DeltaSeconds :type "Float (single-precision)")))

(event `FinishStamina`
  ;[1 1 1] Finish Sprinting
  (bind _returnvalue (`KismetSystemLibrary.K2_SetTimerDelegate` (`|CreateDelegate` :!event `Exhaustion`) 1.0))
  (set `self.Exhausted` _returnvalue))

(event `DecreaseStamina`
  (bind _movementcomponent (`self.MovementComponent`))
  (bind _regainstaminatimerhandle (`self.RegainStaminaTimerHandle`))
  ;[1 1 1] Start Sprinting
  ;;[1 1 1] Decrease Stamina
  (if (> (`KismetMathLibrary.VSize` (`MovementComponent.Velocity` (`self.MovementComponent`))) 0.0)
    (if (`KismetSystemLibrary.K2_IsValidTimerHandle` (`self.Exhausted`))
      (`KismetSystemLibrary.K2_ClearAndInvalidateTimerHandle` (`self.Exhausted`)))
    (if (== (`KismetMathLibrary.FClamp` (`self.CurrentStamina`) 0.0 10000.0) 0.0)
      (`KismetSystemLibrary.K2_ClearAndInvalidateTimerHandle` (`self.DecreaseStaminaTimerHandle`))
      (`self.FinishStamina` :!label _label_2)
      (set `CharacterMovementComponent.MaxWalkSpeed` (/ (`CharacterMovementComponent.MaxWalkSpeed` _movementcomponent) 1.5) _movementcomponent)
      (set `self.Sprinting?` false)
      (else
        (if (`KismetSystemLibrary.K2_IsValidTimerHandle` _regainstaminatimerhandle)
          (`KismetSystemLibrary.K2_ClearAndInvalidateTimerHandle` _regainstaminatimerhandle))
        (set `self.CurrentStamina` (- (`self.CurrentStamina`) 1.0))
        (`self.StaminaModified` (`self.CurrentStamina`) (`self.MaxStamina`))))
    (elif (`self.Button?`)
      (if (not (`KismetSystemLibrary.K2_IsValidTimerHandle` (`self.Exhausted`)))
        (`self.FinishStamina`))
      (else
        (goto _label_2)))))

(event `Exhaustion`
  ;[1 1 1] Finish Sprinting
  ;;[1 1 1] Exhaustion
  (bind _returnvalue (`KismetSystemLibrary.K2_SetTimerDelegate` (`|CreateDelegate` :!event `RegainStamina`) 0.1 true))
  (set `self.RegainStaminaTimerHandle` _returnvalue))

(event `RegainStamina`
  ;[1 1 1] Finish Sprinting
  ;;[1 1 1] Regain Stamina
  (if (== (`self.CurrentStamina`) (`self.MaxStamina`))
    (`KismetSystemLibrary.K2_ClearAndInvalidateTimerHandle` (`self.RegainStaminaTimerHandle`))
    (else
      (set `self.CurrentStamina` (+ (`self.CurrentStamina`) 1.0))
      (`self.StaminaModified` (`self.CurrentStamina`) (`self.MaxStamina`)))))