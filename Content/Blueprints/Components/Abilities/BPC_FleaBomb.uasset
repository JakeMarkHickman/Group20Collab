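; Flea bomb ability component that aims with a ground decal, then launches a projectile at the marked spot.
; The first use enables tick, which traces from the camera against WorldStatic and moves a flea-range-sized decal across upward-facing surfaces, removing it otherwise.
; A second use on a valid surface spawns a projectile above the owner toward that location, stops targeting and starts the cooldown that gates reuse.
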(event `self.ReceiveTick`
  (params (DeltaSeconds :type "Float (single-precision)"))
  (bind _returnvalue (`GameplayStatics.GetPlayerCameraManager` 0))
  (bind _returnvalue_2 (`PlayerCameraManager.GetCameraLocation` _returnvalue))
  (bind _decal (`/Game/Materials/BP_Decal.Decal` (`self.Decal`)))
  ;[1 1 1] Traces
  (bind (_outhit _returnvalue_3) (`KismetSystemLibrary.LineTraceSingleForObjects` _returnvalue_2 (+ _returnvalue_2 (* (`KismetMathLibrary.GetForwardVector` (`PlayerCameraManager.GetCameraRotation` _returnvalue)) 1500.0)) (`|MakeArray` "ObjectTypeQuery1" :!type "EObjectTypeQuery Enum")))
  (if _returnvalue_3
    (`/Engine/EditorBlueprintResources/StandardMacros.IsValid` (`self.Decal`)
      (:`Is Valid`
        _)
      (:`Is Not Valid`
        (`self.SpawnDecal`)))
    (bind _output_get (set `self.Hit` _returnvalue_3))
    (set `self.Can Use` _output_get)
    (bind (_bblockinghit _binitialoverlap _time _distance _location _impactpoint _normal) (`GameplayStatics.BreakHitResult` _outhit))
    (bind _output_get_2 (set `self.UpVector` (== _normal (`KismetMathLibrary.Vector_Up`) :`ErrorTolerance` 0.5)))
    (if _output_get_2
      (`SceneComponent.K2_SetWorldLocation` _decal _location false false)
      (set `self.LocationToMove` (`SceneComponent.K2_GetComponentLocation` _decal))
      (else
        (`Actor.K2_DestroyActor` (`self.Decal`))))
    (else
      (`/Engine/EditorBlueprintResources/StandardMacros.IsValid` (`self.Decal`)
        (:`Is Valid`
          (`Actor.K2_DestroyActor` (`self.Decal`)))))))

(event `/Game/Blueprints/Interfaces/BPI_Abilities.UseAbility`
  (bind _decal (`self.Decal`))
  (bind (_abilityname _abilitycooldown _abilitythumbnail _keyprompt _abilitydescription) (break `/Game/Blueprints/Data/s_AbilityData` (`self.AbilityData`)))
  (bind (_abilityname_2 _abilitycooldown_2 _abilitythumbnail_2 _keyprompt_2 _abilitydescription_2) (break `/Game/Blueprints/Data/s_AbilityData` (`self.AbilityData`)))
  (bind (_returnvalue_x _returnvalue_y _returnvalue_z) (`KismetMathLibrary.BreakVector` (`Actor.K2_GetActorLocation` (`self.GetOwner`))))
  ;[1 1 1] UseAbility
  (if (`KismetSystemLibrary.K2_IsValidTimerHandle` (`self.CooldownTimerHandle`))
    _
    (elif (`self.Targeting`)
      ;;[1 1 1] Shooting
      (if (`self.UpVector`)
        (`GameplayStatics.PlaySound2D` "/Game/Assets/Audio/Rat_Audio/RatBite_-_Track_10.RatBite_-_Track_10" 1.0 1.0 0.0 null null)
        (`KismetSystemLibrary.PrintString` (`KismetStringLibrary.Concat_StrStr` _abilityname_2 "_" (`KismetTextLibrary.Conv_TextToString` _abilitydescription_2)) true true (struct :`R` 1.0 :`G` 0.861449 :`A` 1.0))
        (bind _returnvalue (`|SpawnActorFromClass` "/Game/Blueprints/Projectles/BP_BaseProjectile.BP_BaseProjectile_C" (`KismetMathLibrary.MakeTransform` (`KismetMathLibrary.MakeVector` _returnvalue_x _returnvalue_y (+ _returnvalue_z 20.0))) "Undefined" "MultiplyWithRoot" null (`self.Flea Range`) null))
        (`/Game/Blueprints/Projectles/BP_BaseProjectile.Initialise` _returnvalue (`self.LocationToMove`))
        (`self.SetComponentTickEnabled` false)
        (`self.Cooldown`)
        (`KismetSystemLibrary.DelayUntilNextTick`)
        (set `self.Targeting` false)
        (`/Engine/EditorBlueprintResources/StandardMacros.IsValid` _decal
          (:`Is Valid`
            (`Actor.K2_DestroyActor` _decal))))
      (else
        ;;[1 1 1] Targeting
        (`GameplayStatics.PlaySound2D` "/Game/Assets/Audio/Rat_Audio/Squeak/ratnoise_-_Track_3.ratnoise_-_Track_3" 1.0 1.0 0.0 null null)
        (`KismetSystemLibrary.PrintString` (`KismetStringLibrary.Concat_StrStr` _abilityname "_" (`KismetTextLibrary.Conv_TextToString` _abilitydescription)))
        (`self.SetComponentTickEnabled` true)
        (bind _returnvalue_2 (`|SpawnActorFromClass` "/Game/Materials/BP_Decal.BP_Decal_C" (`KismetMathLibrary.MakeTransform` (0.0 0.0 0.0)) "Undefined" "MultiplyWithRoot" null (`self.Flea Range`) null :!label _label))
        (bind _output_get (set `self.Decal` _returnvalue_2))
        (`KismetSystemLibrary.DelayUntilNextTick`)
        (set `self.Targeting` true)))))

(event `SpawnDecal`
  ;[1 1 1] UseAbility
  ;;[1 1 1] Targeting
  (goto _label))