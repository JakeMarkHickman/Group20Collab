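; Ability component that summons rat allies around its owning character.
; When used while the cooldown timer handle is invalid, it spawns a configurable number of BP_RatAllyCharacter actors, then calls Cooldown.
; Each rat takes a random navigable X/Y near the owner and the owner's height and rotation, adjusting for collisions but always spawning.
; The owning character reference is supplied through GetCharacterRef.
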(event `/Game/Blueprints/Interfaces/BPI_Abilities.UseAbility`
  (bind _owningcharacter (`self.OwningCharacter`))
  (bind (_returnvalue_x _returnvalue_y _returnvalue_z) (`KismetMathLibrary.BreakVector` (`Actor.K2_GetActorLocation` _owningcharacter)))
  (if (not (`KismetSystemLibrary.K2_IsValidTimerHandle` (`self.CooldownTimerHandle`)))
    (for _ (range (+ (`self.AmountOfRatsToSpawn`) 1))
      (bind _randomlocation (`NavigationSystemV1.K2_GetRandomLocationInNavigableRadius` (`Actor.K2_GetActorLocation` _owningcharacter) 100.0 null null))
      (`|SpawnActorFromClass` "/Game/Blueprints/Characters/BP_RatAllyCharacter.BP_RatAllyCharacter_C" (`KismetMathLibrary.MakeTransform` (`KismetMathLibrary.MakeVector` (.x _randomlocation) (.y _randomlocation) _returnvalue_z) (`Actor.K2_GetActorRotation` _owningcharacter)) "AdjustIfPossibleButAlwaysSpawn" "MultiplyWithRoot" null null))
    (`self.Cooldown`)))

(event `/Game/Blueprints/Interfaces/BPI_Abilities.GetCharacterRef`
  (params (OwningCharacter :type "/Game/Blueprints/Characters/BP_Rat Object Reference"))
  (set `self.OwningCharacter` OwningCharacter))