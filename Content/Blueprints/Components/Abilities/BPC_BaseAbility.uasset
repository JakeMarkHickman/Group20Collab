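; BPC_BaseAbility is a base ability component that provides shared cooldown handling, with an empty UseAbility event as the entry point.
; Cooldown starts a timer lasting the cooldown time from AbilityData and stores its handle.
; ReplenishAbility clears and invalidates that timer handle.
; BeginPlay is empty, and the remaining debug print nodes are disconnected.
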(event `self.ReceiveBeginPlay`)

(event `/Game/Blueprints/Interfaces/BPI_Abilities.UseAbility`)

(event `Cooldown`
  (bind _returnvalue (`KismetSystemLibrary.K2_SetTimerDelegate` (`|CreateDelegate` :!event `ReplenishAbility`) (`.AbilityCooldown_13_7029698144E06145D64A0BB09442AD11` (break `/Game/Blueprints/Data/s_AbilityData` (`self.AbilityData`)))))
  (set `self.CooldownTimerHandle` _returnvalue))

(event `ReplenishAbility`
  (`KismetSystemLibrary.K2_ClearAndInvalidateTimerHandle` (`self.CooldownTimerHandle`)))