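; Squeek ability component that makes the rat emit a squeak and report a noise event for AI perception.
; On BeginPlay it caches the BP_Rat actor found by class lookup.
; UseAbility, gated by the cooldown timer handle, plays the sound at the rat's location, reports the noise with the rat as instigator, prints a debug string and calls Cooldown.
; A comment marks further AI work as pending.
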(event `self.ReceiveBeginPlay`
  ;[0.04883 0.04943 0.5729] get rat location
  (bind _returnvalue (`GameplayStatics.GetActorOfClass` "/Game/Blueprints/Characters/BP_Rat.BP_Rat_C"))
  (set `self.BP_Rat` _returnvalue))

(event `/Game/Blueprints/Interfaces/BPI_Abilities.UseAbility`
  (bind _bp_rat (`self.BP_Rat`))
  ;[0.7766 0.1511 1] squeek ability - ai stuff to be added once done
  (if (not (`KismetSystemLibrary.K2_IsValidTimerHandle` (`self.CooldownTimerHandle`)))
    (`GameplayStatics.PlaySoundAtLocation` "/Game/Assets/Audio/Rat_Audio/Squeak/ratnoise_-_Track_17.ratnoise_-_Track_17" (`Actor.K2_GetActorLocation` (`self.BP_Rat`)) (struct) 1.0 1.0 0.0 null null null null)
    (`AISense_Hearing.ReportNoiseEvent` (`Actor.K2_GetActorLocation` _bp_rat) 4.0 _bp_rat)
    (`KismetSystemLibrary.PrintString` "squeek!!!!!")
    (`self.Cooldown`)))