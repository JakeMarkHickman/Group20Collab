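; BPC_Stun is an ability component that stuns a villager caught in a short-range sphere around the player controller's location.
; BeginPlay caches all BP_Villager actors and an unused plague doctor reference.
; UseAbility prints the ability data, runs a single-hit, zero-length pawn sphere trace with persistent debug drawing, and compares the hit against cached villagers.
; A matching villager implementing BPI_AI receives SetStateAsStunned.
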(event `self.ReceiveBeginPlay`
  (bind _outactors (`GameplayStatics.GetAllActorsOfClass` "/Game/Blueprints/AI/Pawns/BP_Villager.BP_Villager_C"))
  (set `self.BP_VillagerArray` _outactors)
  (bind _returnvalue (`GameplayStatics.GetActorOfClass` "/Game/Blueprints/AI/Pawns/BP_PlagueDoctor.BP_PlagueDoctor_C"))
  (set `self.BP_PlagueDoctorRef` _returnvalue))

(event `/Game/Blueprints/Interfaces/BPI_Abilities.UseAbility`
  (bind (_abilityname _abilitycooldown _abilitythumbnail _keyprompt _abilitydescription) (break `/Game/Blueprints/Data/s_AbilityData` (`self.AbilityData`)))
  (bind _returnvalue (`Actor.K2_GetActorLocation` (`GameplayStatics.GetPlayerController` 0)))
  (`KismetSystemLibrary.PrintString` (`KismetStringLibrary.Concat_StrStr` _abilityname "_" (`KismetTextLibrary.Conv_TextToString` _abilitydescription)))
  (bind _outhit (`KismetSystemLibrary.SphereTraceSingleForObjects` :`Start` _returnvalue :`End` _returnvalue :`Radius` 100.0 :`ObjectTypes` (`|MakeArray` "ObjectTypeQuery3" :!type "EObjectTypeQuery Enum") :`bTraceComplex` true :`DrawDebugType` "Persistent"))
  (for _array_element (`self.BP_VillagerArray`)
    (bind _output_get (set `self.currentVillager` _array_element))
    (if (== _array_element (`.HitActor` (`GameplayStatics.BreakHitResult` _outhit)))
      (if (`KismetSystemLibrary.DoesImplementInterface` _output_get "/Game/Blueprints/AI/Interfaces/BPI_AI.BPI_AI_C")
        (`/Game/Blueprints/AI/Interfaces/BPI_AI.SetStateAsStunned` _output_get)
        (`KismetSystemLibrary.PrintString` "stunned")))))