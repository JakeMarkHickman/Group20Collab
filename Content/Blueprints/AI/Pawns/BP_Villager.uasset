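; Villager AI pawn in a rat game that can attack or flee from the player, be stunned or infected, and die.
; Sphere overlap, stun and infection events pass state to its AIC_Villager controller, while interface-style getters and a speed setter expose pawn data and movement.
; Montages drive stomp attacks, sword equipping and hit responses, with callbacks signalling completion.
; Death notifies BP_RatGamemode, stops AI logic and ragdolls after the death montage.
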(event `self.ReceiveBeginPlay`
  ;[1 1 1] BeginPlay
  (bind _asaic_villager (cast `/Game/Blueprints/AI/Controllers/AIC_Villager` (`self.GetController`)))
  (set `self.As AIC Villager` _asaic_villager)
  (bind _asbp_rat_gamemode (cast `/Game/Blueprints/GameModes/BP_RatGamemode` (`GameplayStatics.GetGameMode`)))
  (set `self.BP Rat Gamemode` _asbp_rat_gamemode))

(event `Attack`
  ;[1 1 1] Attack
  (`self.K2_SetActorRotation` (`KismetMathLibrary.FindLookAtRotation` (`self.K2_GetActorLocation`) (`self.K2_GetActorLocation` (`GameplayStatics.GetPlayerCharacter` 0))))
  (`|PlayMontage` (`self.Mesh`) "/Game/Characters/Mannequins/Animations/Mixamo/Montage/AM_Stomp.AM_Stomp"
    (:`OnCompleted`
      _)
    (:`OnInterrupted`
      _))
  (`self.OnAttackEnd`))

(event `EquipWeapon`
  ;[1 1 1] EquipWeapom
  (bind _returnvalue (`|SpawnActorFromClass` (`self.WeaponClass`) (`KismetMathLibrary.MakeTransform` (`self.K2_GetActorLocation`)) "Undefined" "MultiplyWithRoot" null null))
  (bind _output_get (set `self.EquippedWeapon` _returnvalue))
  (`self.K2_AttachToComponent` _output_get (`self.Mesh`) "hand_rSocket" "SnapToTarget" "SnapToTarget" "KeepRelative" true)
  (`|PlayMontage` (`self.Mesh`) "/Game/Characters/Mannequins/Animations/Mixamo/Montage/AM_UnsheathSword.AM_UnsheathSword"
    (:`OnCompleted`
      (set `self.IsWeaponEquipped` true)
      (`self.OnEquippedWeapon`))))

(event `UnequipWeapon`
  ;[1 1 1] UnequipWeapon
  (`|PlayMontage` (`self.Mesh`) "/Game/Characters/Mannequins/Animations/Mixamo/Montage/AM_SheathSword.AM_SheathSword"
    (:`OnBlendOut`
      (`self.K2_DestroyActor` (`self.EquippedWeapon`))
      (set `self.IsWeaponEquipped` false)
      (`self.OnUnequippedWeapon`))))

(event `Infected`
  (set `self.IsInfected` true)
  (`/Game/Blueprints/AI/Controllers/AIC_Villager.IsInfected` (`self.As AIC Villager`)))

(event `self.Sphere.OnComponentBeginOverlap`
  (params (OverlappedComponent :type "PrimitiveComponent Object Reference") (OtherActor :type "Actor Object Reference") (OtherComp :type "PrimitiveComponent Object Reference") (OtherBodyIndex :type Integer) (bFromSweep :type Boolean) (SweepResult :type "HitResult Structure (by ref)"))
  (bind _as_aic_villager (`self.As AIC Villager`))
  ;[1 1 1] TouchSense 50/50 Flee/Attack
  (if (== OtherActor (`GameplayStatics.GetPlayerCharacter` 0))
    (if (`self.ShouldAttack`)
      (`/Game/Blueprints/AI/Controllers/AIC_Villager.SetStateAsAttacking` _as_aic_villager OtherActor false)
      (else
        (`/Game/Blueprints/AI/Controllers/AIC_Villager.SetStateAsFleeing` _as_aic_villager)))))

(event `/Game/Blueprints/AI/Interfaces/BPI_AI.SetStateAsStunned`
  ;[1 1 1] On Stunned
  (`/Game/Blueprints/AI/Controllers/AIC_Villager.SetStateAsStunned` (`self.As AIC Villager`))
  (`NiagaraFunctionLibrary.SpawnSystemAttached` "/Game/Particles/N_StunHalo.N_StunHalo" (`self.Mesh`) "None" (0.0 0.0 175.0) (struct) "KeepRelativeOffset")
  (`GameplayStatics.PlaySoundAtLocation` "/Game/Assets/Audio/NPC/NPConStun.NPConStun" (`self.K2_GetActorLocation`) (struct) 10.0 1.0 0.0 null null null null))

(event `/Game/Blueprints/AI/Interfaces/BPI_AI.SetStateAsDamaged`
  ;[1 1 1] On Hit
  (`|PlayMontage` (`self.Mesh`) "/Game/Characters/Mannequins/Animations/Mixamo/Montage/AM_HitResponse.AM_HitResponse"
    (:`then`
      (`self.Infected`)
      (`KismetSystemLibrary.Delay` 0.2)
      (`GameplayStatics.PlaySoundAtLocation` "/Game/Assets/Audio/NPC/NPConBite.NPConBite" (`self.K2_GetActorLocation`) (struct) 0.5 1.0 0.0 null null null null)
      (`KismetSystemLibrary.PrintString` "Hello"))))

(event `self.Health._OnDeath`
  (params (Instigator :type "Controller Object Reference"))
  (bind _mesh (`self.Mesh`))
  ;[1 1 1] Stop Behaviour Tree
  (`/Game/Blueprints/GameModes/BP_RatGamemode.E_VillagerDied` (`self.BP Rat Gamemode`))
  (`BrainComponent.StopLogic` (`AIController.BrainComponent` (`self.As AIC Villager`)) "")
  ;[1 1 1] Death Anim
  (`|PlayMontage` (`self.Mesh`) "/Game/Blueprints/AI/Pawns/Animation/Villager/AM_Death_V1.AM_Death_V1"
    (:`OnBlendOut`
      ;[1 1 1] Ragdoll
      (`PrimitiveComponent.SetSimulatePhysics` _mesh true)
      (`PrimitiveComponent.SetCollisionEnabled` _mesh "QueryAndPhysics"))
    (:`OnNotifyBegin`
      ;[1 1 1] Stop Moving/Sliding
      (`MovementComponent.StopMovementImmediately` (`self.CharacterMovement`)))))

(fn `GetIdealRange`
  (returns (MeleeAttackRadius :type "Float (double-precision)") (RangedAttackRadius :type "Float (double-precision)"))
  (return 0.0 0.0))

(fn `GetPatrolRoute`
  (returns (PatrolRoute :type "/Game/Blueprints/AI/PatrolRoute/BP_PatrolRoute Object Reference"))
  (return (`self.PatrolRoute`)))

(fn `GetRef_PD`
  (returns (BP_PlagueDoctor :type "/Game/Blueprints/AI/Pawns/BP_PlagueDoctor Object Reference"))
  (return null))

(fn `GetRef_V`
  (returns (BP_VIllager :type "/Game/Blueprints/AI/Pawns/BP_Villager Object Reference"))
  (return self))

(fn `SetMovementSpeed`
  (params (Speed :type "/Game/Blueprints/AI/Enums/E_MovementSpeed Enum" :default "NewEnumerator0") (Modifier :type "Float (double-precision)"))
  (returns (SpeedValue :type "Float (double-precision)"))
  (bind _output_get (set `CharacterMovementComponent.MaxWalkSpeed` (* Modifier (select `/Game/Blueprints/AI/Enums/E_MovementSpeed` Speed :`NewEnumerator1` 100.0 :`NewEnumerator2` 300.0 :`NewEnumerator3` 500.0 :!type "Float (single-precision)")) (`self.CharacterMovement`)))
  (return _output_get))

(fn `UserConstructionScript`)