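; Plague Doctor enemy pawn, driven by AIC_PlagueDoctor, with melee, grab and thrown-grenade attacks plus a stun reaction.
; Attack montages pause further attacks, move the lamp to the hip and turn the pawn toward the player on a looping timer.
; A hand-socket sphere trace damages or attaches the player by attack type; grab victims are released and damaged when the montage ends.
; Getters supply attack ranges and patrol route, and SetMovementSpeed maps states to walk speeds.
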(event `StopRotation`
  ;[1 1 1] Stop Rotation
  (`KismetSystemLibrary.K2_ClearAndInvalidateTimerHandle` (`self.RotatingTimerHandle`))
  (set `CharacterMovementComponent.bOrientRotationToMovement` true (`self.CharacterMovement`)))

(event `StopAnimation`
  ;[1 1 1] Stop Grab
  (`KismetSystemLibrary.Delay` 1.1)
  (`self.StopAnimMontage` (`self.AM_Grab`)))

(event `/Game/Blueprints/AI/Interfaces/BPI_AI.SetStateAsStunned`
  ;[1 0 0.0378] OnStunned
  (message `/Game/Blueprints/AI/Interfaces/BPI_AI.SetStateAsStunned` (`self.As AIC Plague Doctor`))
  (`CharacterMovementComponent.SetMovementMode` (`self.CharacterMovement`) "MOVE_None" 0)
  (`|PlayMontage` (`self.Mesh`) "/Game/Blueprints/AI/Pawns/Animation/PlagueDoctor/Animations/AM_PD_Stun.AM_PD_Stun" 0.9
    (:`OnCompleted`
      _)
    (:`OnInterrupted`
      _))
  (`self.OnAttackEnd`)
  (`KismetSystemLibrary.Delay` 0.2)
  (`CharacterMovementComponent.SetMovementMode` (`self.CharacterMovement`) "MOVE_Walking" 0))

(event `self.ReceiveBeginPlay`
  ;[1 1 1] BeginPlay
  (bind _asaic_plague_doctor (cast `/Game/Blueprints/AI/Controllers/AIC_PlagueDoctor` (`self.GetController`)))
  (set `self.As AIC Plague Doctor` _asaic_plague_doctor)
  (set `self.IsWeaponEquipped` true)
  (`self.OnEquippedWeapon`))

(event `HandlePlayer`
  ;[1 1 1] HandleCaughtPlayer
  (`self.K2_DetachFromActor` (`self.Hit Actor`) "KeepWorld" "KeepWorld" "KeepWorld")
  (`CharacterMovementComponent.SetMovementMode` (`self.GetComponentByClass` (`self.Hit Actor`) "/Script/Engine.CharacterMovementComponent") "MOVE_Walking" 0)
  (`GameplayStatics.ApplyDamage` (`self.Hit Actor`) (`self.DamageAmount`) null self))

(event `Long Range AOE`
  (params (AttackTarget :type "Actor Object Reference"))
  ;[0 0.3943 1] Long Range Attack
  (set `self.Attack Target` AttackTarget)
  (set `self.E_PD_AttackTypes` "NewEnumerator1")
  (`|PlayMontage` (`self.Mesh`) "/Game/Blueprints/AI/Pawns/Animation/PlagueDoctor/Animations/AM_PD_SmokeBomb.AM_PD_SmokeBomb"
    (:`then`
      (`self.RotateTimer`)
      (set `CharacterMovementComponent.bOrientRotationToMovement` false (`self.CharacterMovement`))
      (set `self.bCanAttack?` false)
      (`self.MoveLampToHip`))
    (:`OnBlendOut`
      (`self.OnAttackEnd` :!label _label)
      (`KismetSystemLibrary.K2_ClearAndInvalidateTimerHandle` (`self.RotatingTimerHandle`))
      (set `CharacterMovementComponent.bOrientRotationToMovement` true (`self.CharacterMovement`))
      (set `self.bCanAttack?` true))
    (:`OnInterrupted`
      (goto _label))
    (:`OnNotifyBegin`
      (`self.SpawnGrenade`))))

(event `StartTrace`
  (bind _returnvalue (`SceneComponent.GetSocketLocation` (`self.Mesh`) "S_Grenade"))
  ;[1 1 1] Trace for Dmg Or Grab
  (bind (_outhit _returnvalue_2) (`KismetSystemLibrary.SphereTraceSingleForObjects` _returnvalue _returnvalue 60.0 (`|MakeArray` "ObjectTypeQuery3" :!type "EObjectTypeQuery Enum")))
  (if _returnvalue_2
    (bind (_bblockinghit _binitialoverlap _time _distance _location _impactpoint _normal _impactnormal _physmat _hitactor) (`GameplayStatics.BreakHitResult` _outhit))
    (set `self.Hit Actor` _hitactor)
    (if (== (`GameplayStatics.GetPlayerCharacter` 0) _hitactor)
      (switch `/Game/Blueprints/AI/Pawns/E_PD_AttackTypes` (`self.E_PD_AttackTypes`)
        (:`NewEnumerator0`
          (`GameplayStatics.ApplyDamage` (`self.Hit Actor`) 25.0 null self))
        (:`NewEnumerator2`
          (`self.SnapPlayerToHand`))))
    (else
      (`self.StopAnimation`))))

(event `StandardAttack`
  ;[0 0.3943 1] Attack
  (`CharacterMovementComponent.SetMovementMode` (`self.CharacterMovement`) "MOVE_None" 0)
  (set `self.E_PD_AttackTypes` "NewEnumerator0")
  (`self.RotateToTargetActor`)
  (`|PlayMontage` (`self.Mesh`) "/Game/Blueprints/AI/Pawns/Animation/PlagueDoctor/Animations/AM_PD_GrabKill.AM_PD_GrabKill"
    (:`then`
      (`self.RotateTimer`)
      (set `CharacterMovementComponent.bOrientRotationToMovement` false (`self.CharacterMovement`))
      (set `self.bCanAttack?` false)
      (`self.MoveLampToHip`))
    (:`OnCompleted`
      (`self.OnAttackEnd` :!label _label_2)
      (`CharacterMovementComponent.SetMovementMode` (`self.CharacterMovement`) "MOVE_Walking" 0)
      (`KismetSystemLibrary.K2_ClearAndInvalidateTimerHandle` (`self.RotatingTimerHandle`))
      (set `CharacterMovementComponent.bOrientRotationToMovement` true (`self.CharacterMovement`))
      (set `self.bCanAttack?` true))
    (:`OnInterrupted`
      (goto _label_2))))

(event `MoveLampToHand`
  ;[1 1 1] Sockets
  (`SceneComponent.K2_AttachToComponent` (`self.SM_Lamp`) (`self.Mesh`) "S_LampHand" "SnapToTarget" "SnapToTarget" "SnapToTarget" true))

(event `MoveLampToHip`
  ;[1 1 1] Sockets
  (`SceneComponent.K2_AttachToComponent` (`self.SM_Lamp`) (`self.Mesh`) "S_LampWaist" "SnapToTarget" "SnapToTarget" "SnapToTarget" true))

(event `RotateTimer`
  ;[1 1 1] Rotate
  (bind _returnvalue (`KismetSystemLibrary.K2_SetTimerDelegate` (delegate `Rotate`) 0.01 true true))
  (set `self.RotatingTimerHandle` _returnvalue))

(event `Rotate`
  ;[1 1 1] Rotate
  (if (`KismetSystemLibrary.K2_IsValidTimerHandle` (`self.RotatingTimerHandle`))
    (`self.RotateToTargetActor`)))

(event `GrabAttack`
  ;[0 0.3943 1] Grab Attack
  (`CharacterMovementComponent.SetMovementMode` (`self.CharacterMovement`) "MOVE_None" 0)
  (set `self.E_PD_AttackTypes` "NewEnumerator2")
  (`|PlayMontage` (`self.Mesh`) (`self.AM_Grab`)
    (:`then`
      (`self.RotateTimer`)
      (set `CharacterMovementComponent.bOrientRotationToMovement` false (`self.CharacterMovement`))
      (set `self.bCanAttack?` false)
      (`self.MoveLampToHip`))
    (:`OnCompleted`
      (`self.OnAttackEnd` :!label _label_3)
      (`CharacterMovementComponent.SetMovementMode` (`self.CharacterMovement`) "MOVE_Walking" 0)
      (`KismetSystemLibrary.K2_ClearAndInvalidateTimerHandle` (`self.RotatingTimerHandle`))
      (set `CharacterMovementComponent.bOrientRotationToMovement` true (`self.CharacterMovement`))
      (set `self.bCanAttack?` true)
      (`/Engine/EditorBlueprintResources/StandardMacros.IsValid` (`self.Hit Actor`)
        (:`Is Valid`
          (`self.HandlePlayer`))))
    (:`OnInterrupted`
      (goto _label_3))
    (:`OnNotifyBegin`
      (`self.StopAnimation`))))

(event `SnapPlayerToHand`
  ;[1 1 1] Snap Player To Hand
  (`/Engine/EditorBlueprintResources/StandardMacros.IsValid` (`self.Hit Actor`)
    (:`Is Valid`
      (`self.K2_AttachToComponent` (`self.Hit Actor`) (`self.Mesh`) "S_Grenade" "SnapToTarget" "SnapToTarget" "KeepWorld" true)
      (`CharacterMovementComponent.SetMovementMode` (`self.GetComponentByClass` (`self.Hit Actor`) "/Script/Engine.CharacterMovementComponent") "MOVE_None" 0))))

(event `SpawnGrenade`
  ;[1 1 1] Spawn Grenade
  (`|SpawnActorFromClass` "/Game/Blueprints/Weapons/BP_RatRepellantGrenade.BP_RatRepellantGrenade_C" (`KismetMathLibrary.MakeTransform` (`SceneComponent.GetSocketLocation` (`self.Mesh`) "S_Grenade")) "Undefined" "MultiplyWithRoot" self (`self.Attack Target`) (`self.BP_Rat`) null))

(fn `GetIdealRange`
  (returns (MeleeAttackRadius :type "Float (double-precision)") (RangedAttackRadius :type "Float (double-precision)"))
  (return 100.0 600.0))

(fn `GetPatrolRoute`
  (returns (PatrolRoute :type "/Game/Blueprints/AI/PatrolRoute/BP_PatrolRoute Object Reference"))
  (return (`self.PatrolRoute`)))

(fn `GetRef_PD`
  (returns (BP_PlagueDoctor :type "/Game/Blueprints/AI/Pawns/BP_PlagueDoctor Object Reference"))
  (return self))

(fn `GetRef_V`
  (returns (BP_VIllager :type "/Game/Blueprints/AI/Pawns/BP_Villager Object Reference"))
  (return null))

(fn `IsClaimed`
  (returns (bIsClaimed :type Boolean))
  (return false))

(fn `RotateToTargetActor`
  (bind (_returnvalue_roll _returnvalue_pitch _returnvalue_yaw) (`KismetMathLibrary.BreakRotator` (`KismetMathLibrary.FindLookAtRotation` (`self.K2_GetActorLocation`) (`self.K2_GetActorLocation` (`GameplayStatics.GetPlayerCharacter` 0)))))
  ;[1 1 1] Rotate to Target (Does once)
  (`self.K2_SetActorRotation` (`KismetMathLibrary.MakeRotator` 0.0 0.0 _returnvalue_yaw)))

(fn `SetMovementSpeed`
  (params (Speed :type "/Game/Blueprints/AI/Enums/E_MovementSpeed Enum" :default "NewEnumerator0") (Modifier :type "Float (double-precision)"))
  (returns (SpeedValue :type "Float (double-precision)"))
  (bind _output_get (set `CharacterMovementComponent.MaxWalkSpeed` (select `/Game/Blueprints/AI/Enums/E_MovementSpeed` Speed :`NewEnumerator1` 80.0 :`NewEnumerator2` 150.0 :`NewEnumerator3` 200.0 :!type "Float (single-precision)") (`self.CharacterMovement`)))
  (return _output_get))

(fn `UserConstructionScript`
  (`SceneComponent.K2_AttachToComponent` (`self.SM_Scythe`) (`self.Mesh`) "S_Scythe" "KeepRelative" "KeepRelative" "KeepRelative" true)
  (`SceneComponent.K2_AttachToComponent` (`self.SM_Lamp`) (`self.Mesh`) "S_Lamp" "KeepRelative" "KeepRelative" "KeepRelative" true))