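; Villager component that shows health through a colour-changing N_Health Niagara effect.
; On BeginPlay it attaches the system to the owning BP_Villager's root and binds to health-change and status-effect events.
; UpdateColour blends between low and high health colours using a clamped remap of the health ratio.
; BeginParticles and EndParticles toggle the effect and refresh its colour, while CustomEvent, which takes an effect, is an empty stub.
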(event `self.ReceiveBeginPlay`
  ;[1 1 1] Init Owning Character Variable
  (bind _asbp_villager (cast `/Game/Blueprints/AI/Pawns/BP_Villager` (`self.GetOwner`)))
  (bind _output_get (set `self.Owner Ref` _asbp_villager))
  ;[1 1 1] Spawns the particle
  (bind _returnvalue (`NiagaraFunctionLibrary.SpawnSystemAttached` "/Game/Blueprints/AI/Particles/N_Health.N_Health" (`Actor.RootComponent` _output_get) "None" (0.0 0.0 0.0) (struct) "KeepRelativeOffset"))
  (set `self.Particle` _returnvalue)
  ;[1 1 1] Bind to Health Changing
  (add `HealthComponent._OnHealthChanged` (`/Game/Blueprints/AI/Pawns/BP_Villager.Health` (`self.Owner Ref`)) (`|CreateDelegate` :!event `UpdateColour`))
  ;[1 0 0] Bind to Status Effects
  (add `StatusEffectComponent._OnStatusEffectAdded` (`/Game/Blueprints/AI/Pawns/BP_Villager.StatusEffect` (`self.Owner Ref`)) (`|CreateDelegate` :!event `CustomEvent`)))

(event `Begin Particles`
  ;[1 1 1] Activate/Deactivate
  (`self.Activate` (`self.Particle`) false)
  (`self.UpdateColour` (`HealthComponent.GetCurrentHealth` (`/Game/Blueprints/AI/Pawns/BP_Villager.Health` (`self.Owner Ref`)))))

(event `UpdateColour`
  (params (UpdatedHealth :type "Float (single-precision)") (HealthChanged :type "Float (single-precision)") (Instigator :type "Controller Object Reference"))
  ;[1 1 1] Change Colour On Health Change
  (`NiagaraComponent.SetVariableLinearColor` (`self.Particle`) "Colour" (`KismetMathLibrary.LinearColorLerp` (`self.lowHealthColour`) (`self.highHealthColour`) (`KismetMathLibrary.MapRangeClamped` (/ UpdatedHealth (`HealthComponent.GetMaxHealth` (`/Game/Blueprints/AI/Pawns/BP_Villager.Health` (`self.Owner Ref`)))) 0.1 0.8 0.0 1.0))))

(event `End Particles`
  ;[1 1 1] Activate/Deactivate
  (`self.Deactivate` (`self.Particle`))
  (`self.UpdateColour` (`HealthComponent.GetCurrentHealth` (`/Game/Blueprints/AI/Pawns/BP_Villager.Health` (`self.Owner Ref`)))))

(event `CustomEvent`
  (params (effect :type "BaseStatusEffect Class Reference")))