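; Spawn manager that adds plague doctor enemies to the rat game, up to a configured cap.
; BeginPlay caches the player rat and binds to the game mode's villager-infected event.
; AttemptSpawn rolls a spawn chance, then places a doctor at the Spawners entry farthest from the rat, using a maximum distance that is never reset between attempts.
; The first spawn also notifies the rat once.
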(event `self.ReceiveBeginPlay`
  (bind _asbp_rat_gamemode (cast `/Game/Blueprints/GameModes/BP_RatGamemode` (`GameplayStatics.GetGameMode`)))
  (bind _returnvalue (`GameplayStatics.GetActorOfClass` "/Game/Blueprints/Characters/BP_Rat.BP_Rat_C"))
  (set `self.PlayerRat` _returnvalue)
  (add `/Game/Blueprints/GameModes/BP_RatGamemode.E_VillagerInfected` _asbp_rat_gamemode (`|CreateDelegate` :!event `Attempt Spawn`)))

(event `Attempt Spawn`
  (if (>= (`self.MaxPlagueDoctors`) (`self.SpawnedDoctors`))
    (if (<= (`KismetMathLibrary.RandomFloat`) (`self.Spawn Chance`))
      (for _array_element (`self.Spawners`)
        (bind _returnvalue (`SceneComponent.K2_GetComponentLocation` (`Actor.RootComponent` _array_element)))
        (bind _returnvalue_2 (`KismetMathLibrary.Vector_Distance` _returnvalue (`SceneComponent.K2_GetComponentLocation` (`Actor.RootComponent` (`self.PlayerRat`)))))
        (if (> _returnvalue_2 (`self.FurthestLocation`))
          (set `self.FurthestLocation` _returnvalue_2)
          (set `self.ChosenSpawn` _returnvalue)))
      (`/Engine/EditorBlueprintResources/StandardMacros.IncrementInt` (`self.SpawnedDoctors`)
        (:`  `
          (`|SpawnActorFromClass` "/Game/Blueprints/AI/Pawns/BP_PlagueDoctor.BP_PlagueDoctor_C" (`KismetMathLibrary.MakeTransform` (`self.ChosenSpawn`)) "Undefined" "MultiplyWithRoot" null "/Game/Blueprints/Weapons/BP_Weapon.BP_Weapon_C" null 50.0 null)
          (`/Engine/EditorBlueprintResources/StandardMacros.DoOnce` false
            (:`Completed`
              (`/Game/Blueprints/Characters/BP_Rat.FirstDoctorSpawned` (`self.PlayerRat`)))))))))

(fn `UserConstructionScript`)