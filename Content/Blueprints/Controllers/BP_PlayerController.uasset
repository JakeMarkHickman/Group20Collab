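; Player controller that creates the main HUD and pause menu on BeginPlay and routes the player's Enhanced Input actions.
; Flea Bomb, Stun and Rat Allies inputs each find their ability component on the controlled pawn and send it a UseAbility interface message.
; Sprint start and end go to the pawn as messages, while the pause input triggers the stored pause menu widget.
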(event `EnhancedInput|/Game/Blueprints/Controls/Inputs/IA_FleaBomb`
  (params (ActionValue :type Boolean) (ElapsedSeconds :type "Float (double-precision)") (TriggeredSeconds :type "Float (double-precision)") (InputAction :type "InputAction Object Reference" :default "/Game/Blueprints/Controls/Inputs/IA_FleaBomb.IA_FleaBomb"))
  ;[1 1 1] Abilities
  (:`Started`
    (message `/Game/Blueprints/Interfaces/BPI_Abilities.UseAbility` (`self.GetComponentByClass` (`self.K2_GetPawn`) "/Game/Blueprints/Components/Abilities/BPC_FleaBomb.BPC_FleaBomb_C"))))

(event `EnhancedInput|/Game/Blueprints/Controls/Inputs/IA_Stun`
  (params (ActionValue :type Boolean) (ElapsedSeconds :type "Float (double-precision)") (TriggeredSeconds :type "Float (double-precision)") (InputAction :type "InputAction Object Reference" :default "/Game/Blueprints/Controls/Inputs/IA_Stun.IA_Stun"))
  ;[1 1 1] Abilities
  (:`Started`
    (message `/Game/Blueprints/Interfaces/BPI_Abilities.UseAbility` (`self.GetComponentByClass` (`self.K2_GetPawn`) "/Game/Blueprints/Components/Abilities/BPC_Stun.BPC_Stun_C"))))

(event `EnhancedInput|/Game/Blueprints/Controls/Inputs/IA_RatAllies`
  (params (ActionValue :type Boolean) (ElapsedSeconds :type "Float (double-precision)") (TriggeredSeconds :type "Float (double-precision)") (InputAction :type "InputAction Object Reference" :default "/Game/Blueprints/Controls/Inputs/IA_RatAllies.IA_RatAllies"))
  ;[1 1 1] Abilities
  (:`Started`
    (message `/Game/Blueprints/Interfaces/BPI_Abilities.UseAbility` (`self.GetComponentByClass` (`self.K2_GetPawn`) "/Game/Blueprints/Components/Abilities/BPC_RatAllies.BPC_RatAllies_C"))))

(event `self.ReceiveBeginPlay`
  (bind _returnvalue (`|CreateWidget` "/Game/UI/MainHUD/WBP_MainHUD.WBP_MainHUD_C"))
  (`UserWidget.AddToViewport` _returnvalue 0)
  (bind _returnvalue_2 (`|CreateWidget` "/Game/UI/PauseMenu/WBP_PauseMenu.WBP_PauseMenu_C"))
  (bind _output_get (set `self.PauseMenu` _returnvalue_2))
  (`UserWidget.AddToViewport` _output_get 0))

(event `EnhancedInput|/Game/Blueprints/Controls/Inputs/IA_Sprint`
  (params (ActionValue :type Boolean) (ElapsedSeconds :type "Float (double-precision)") (TriggeredSeconds :type "Float (double-precision)") (InputAction :type "InputAction Object Reference" :default "/Game/Blueprints/Controls/Inputs/IA_Sprint.IA_Sprint"))
  (bind _returnvalue (`self.K2_GetPawn`))
  (:`Started`
    (message `/Game/Blueprints/Interfaces/BPI_Sprint.StartSprint` _returnvalue))
  (:`Completed`
    (message `/Game/Blueprints/Interfaces/BPI_Sprint.EndSprint` _returnvalue)))

(event `EnhancedInput|/Game/Blueprints/Controls/Inputs/IA_TrigPause`
  (params (ActionValue :type Boolean) (ElapsedSeconds :type "Float (double-precision)") (TriggeredSeconds :type "Float (double-precision)") (InputAction :type "InputAction Object Reference" :default "/Game/Blueprints/Controls/Inputs/IA_TrigPause.IA_TrigPause"))
  (:`Triggered`
    (`/Game/UI/PauseMenu/WBP_PauseMenu.TriggerPause` (`self.PauseMenu`))))

(fn `UserConstructionScript`)